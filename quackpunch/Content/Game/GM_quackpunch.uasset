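; Game mode for quackpunch that runs a sequence of three enemies and handles the win.
; SpawnEnemies, first run at BeginPlay, spawns one enemy with a default controller, passes its reference to the player character and increments EnemiesKilled at spawn time.
; A call made once that counter equals three fires the Win dispatcher instead, which spawns a Niagara effect and opens the menu level after a delay.
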(event Custom|Event%20Win
  (Niagara|SpawnSystematLocation "/Game/Win/NS_Win.NS_Win" "0.000000,0.000000,100.000000")
  (Utilities|FlowControl|Delay 5.0)
  (Game|OpenLevel(byObjectReference) "/Game/Maps/Menu.Menu"))

(event EventBeginPlay
  (EventDispatchers|BindEventtoWin (delegate Custom|Event%20Win))
  (CallFunction|SpawnEnemies))

(fn ConstructionScript)

(fn SpawnEnemies
  (if (== (Variables|Data|GetEnemiesKilled) 3)
    (Default|CallWin)
    (else
      (bind _returnvalue (Game|SpawnActorfromClass "/Game/Game/Enemies/C_Enemies.C_Enemies_C" (Math|Transform|MakeTransform "100.000000,0.000000,500.000000" "0, 0, 0" "1.000000,1.000000,1.000000") "AdjustIfPossibleButAlwaysSpawn" 0 0))
      (Pawn|SpawnDefaultController _returnvalue)
      (bind _asc_quackpunch (Utilities|Casting|CastToC_quackpunch (Game|GetPlayerCharacter 0)))
      (Variables|/Game/Game/Player/C_quackpunch.C_quackpunch_C|SetEnemieRef _asc_quackpunch _returnvalue)
      (Math|Integer|IncrementInt (Variables|Data|GetEnemiesKilled)))))