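; BP_Camera is the game camera actor that becomes the player's view target and follows the player character.
; On BeginPlay it fades the screen in over FadeDuration and takes over the view, then stops the fade after a matching delay.
; Each tick it smoothly interpolates its location toward the C_quackpunch character's position with VInterpTo, changing only location and never rotation.
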(event EventTick
  (params (DeltaSeconds :type Float%20%28single-precision%29))
  (bind _asc_quackpunch (Utilities|Casting|CastToC_quackpunch (Game|GetPlayerCharacter 0)))
  (Variables|Default|SetCameraTargetLocation (Transformation|GetActorLocation _asc_quackpunch))
  (bind _output_get (Variables|Default|SetCameraCurrentLocation (Math|Interpolation|VInterpTo (Variables|Default|GetCameraCurrentLocation) (Variables|Default|GetCameraTargetLocation) (Utilities|Time|GetWorldDeltaSeconds) 5.0)))
  (Transformation|SetActorLocation _output_get false false))

(event EventBeginPlay
  (bind _returnvalue (Game|GetPlayerCameraManager 0))
  (bind _fadeduration (Variables|Default|GetFadeDuration))
  (CameraFades|StartCameraFade :self _returnvalue :FromAlpha 1.0 :ToAlpha 0.0 :Duration _fadeduration)
  (Utilities|FlowControl|Sequence
    (:then_0
      (Game|Player|SetViewTargetwithBlend (Game|GetPlayerController 0) self 0.0 "VTBlend_Linear" 0.0 true))
    (:then_1
      (Utilities|FlowControl|Delay _fadeduration)
      (CameraFades|StopCameraFade _returnvalue))))

(fn ConstructionScript)